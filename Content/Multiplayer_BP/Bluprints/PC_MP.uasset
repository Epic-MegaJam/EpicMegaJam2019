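; PC_MP is a multiplayer player controller that manages the local player's HUD widget.
; ClientPostLogin calls SetupGameHud, which creates W_MPHUD only for a local controller, stores it and adds it to the viewport.
; It then casts the game mode to MO_GM without using the result.
; EndPlay removes the HUD from its parent.
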(event `ClientPostLogin`
  (`self.SetupGameHud`)
  (cast `/Game/Multiplayer_BP/Bluprints/MO_GM` (`GameplayStatics.GetGameMode`)))

(event `self.ReceiveEndPlay`
  (params (EndPlayReason :type "EEndPlayReason Enum" :default "Destroyed"))
  (`Widget.RemoveFromParent` (`self.W_HUD`)))

(fn `SetupGameHud`
  (if (`self.IsLocalPlayerController`)
    (bind _returnvalue (`|CreateWidget` "/Game/Multiplayer_BP/Widgets/W_MPHUD.W_MPHUD_C" self))
    (bind _output_get (set `self.W_HUD` _returnvalue))
    (`UserWidget.AddToViewport` _output_get 0)))

(fn `UserConstructionScript`)